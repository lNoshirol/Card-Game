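; BP_SetCard builds the player's card hand from the DT_Cards data table on BeginPlay.
; It creates a W_Card widget with each row's image and collects them in a list.
; After a short delay it copies the list to a backup, then repeatedly moves a random card from the list into the HUD's WCardHand, so no widget is drawn twice.
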(event EventBeginPlay
  (bind _outrownames (DataTable|GetDataTableRowNames "/Game/Level/BP/CardHand/DT_Cards.DT_Cards"))
  (for _array_element _outrownames
    (bind _returnvalue (Utilities|GetDataTableRow "/Game/Level/BP/CardHand/DT_Cards.DT_Cards" _array_element)
      (:then
        (bind _returnvalue_2 (UserInterface|CreateWidget "/Game/Level/BP/CardHand/W_Card.W_Card_C" 0 (Utilities|Struct|MakeS_CardInfo (.Image (Utilities|Struct|BreakS_CardInfo _returnvalue)) 0 "")))
        (Utilities|Array|Add (Variables|Default|GetListCard) _returnvalue_2))))
  (Utilities|FlowControl|Delay 0.2)
  (Variables|Default|SetW_Card_Hand (Variables|/Game/Level/BP/CardHand/W_CardHUD.W_CardHUD_C|GetW_CardHand (Variables|Default|GetCardHUD)))
  (for _array_element_2 (Variables|Default|GetListCard)
    (Utilities|Array|Add (Variables|Default|GetListCardBackUp) _array_element_2))
  (for _index (range 1 (Variables|Default|GetLast%20Index))
    (bind _output_get (Variables|Default|SetGetInfo (.OutItem (Utilities|Array|Random (Variables|Default|GetListCard)))))
    (Utilities|Array|RemoveItem (Variables|Default|GetListCard) _output_get)
    (Class|BPAddCard|AddCard(Message) (Variables|Default|GetW_Card_Hand) _output_get)))

(fn ConstructionScript)